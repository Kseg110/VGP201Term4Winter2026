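; Health component that stores an actor's health, clamped between min and max, with damage, heal, reset and death checks.
; Damage and Heal reject non-positive amounts and route changes through SetHealth, which applies the clamp.
; The CustomDamage event applies damage and, on zero health, fires the owning BP_Player's death message and triggers game over on BP_GameManager.
; Debug prints report health and errors.
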(event Custom|CustomDamage
  (params (DamageAmt :type Float%20%28double-precision%29))
  (CallFunction|Damage DamageAmt)
  (if (CallFunction|IsDead)
    (Development|PrintString "Health Is Zero" true true "(R=1.000000,G=0.871599,B=0.261077,A=1.000000)" 5.0)
    (Utilities|FlowControl|DoOnce false
      (:Completed
        (bind _asbp_player (Utilities|Casting|CastToBP_Player (Components|GetOwner)))
        (Class|BPIGameControl|OnDeathTrigger(Message) _asbp_player)
        (Development|PrintString "Calling Game Over" true true "(R=1.000000,G=0.862883,B=0.223958,A=1.000000)" 5.0)
        (bind _asbp_game_manager (Utilities|Casting|CastToBP_GameManager (Game|GetGameMode)))
        (Default|TriggerGameOver _asbp_game_manager 0.0)))))

(event EventBeginPlay
  (CallFunction|PrintHealth))

(fn Reset
  (Variables|Default|SetHealth (Variables|Default|GetMaxHealth)))

(fn GetHealth
  (return (Variables|Default|GetHealth)))

(fn SetHealth
  (params (NewHeatlh :type Float%20%28double-precision%29))
  (bind _output_get (Variables|Default|SetHealth (CallFunction|ClampHealth NewHeatlh)))
  (return _output_get))

(fn PrintHealth
  (Development|PrintString (Utilities|String|ToString(Float) (CallFunction|GetHealth)) true true "(R=1.000000,G=0.176820,B=0.885851,A=1.000000)"))

(fn ClampHealth
  (params (Value :type Float%20%28double-precision%29))
  (return (Math|Float|Clamp(Float) Value (Variables|Default|GetMinHealth) (Variables|Default|GetMaxHealth))))

(fn Damage
  (params (DamageAmt :type Float%20%28double-precision%29))
  (if (> DamageAmt 0.0)
    (CallFunction|SetHealth (- (CallFunction|GetHealth) DamageAmt))
    (else
      (Development|PrintString "Damage value must be positive +" true true "(R=1.000000,G=0.072917,B=0.072917,A=1.000000)" 6.0))))

(fn Heal
  (params (HealAmt :type Float%20%28double-precision%29))
  (if (> HealAmt 0.0)
    (CallFunction|SetHealth (+ (CallFunction|GetHealth) HealAmt))
    (else
      (Development|PrintString "Healing value must be positive +" true true "(R=0.376054,G=1.000000,B=0.352321,A=1.000000)" 6.0))))

(fn HealFull
  (CallFunction|Heal 1e+02))

(fn Killed
  (CallFunction|Damage 1e+02))

(fn GetNormalizedHealth
  (return (Math|Float|Clamp(Float) (/ (CallFunction|GetHealth) (Variables|Default|GetHealth)) 0.0 (Variables|Default|GetMaxHealth))))

(fn IsDead
  (return (<= (CallFunction|GetHealth) 0.0)))

(fn Init
  (params (Health :type Float%20%28double-precision%29) (MinHealth :type Float%20%28double-precision%29) (MaxHealth :type Float%20%28double-precision%29))
  (CallFunction|SetHealth Health)
  (Variables|Default|SetMinHealth MinHealth)
  (Variables|Default|SetMaxHealth MaxHealth))