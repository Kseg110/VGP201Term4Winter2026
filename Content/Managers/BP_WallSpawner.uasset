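; Timed spawner actor that creates actors from the EnemyPool class list at a fixed interval.
; BeginPlay starts a looping timer that fires the SpawnWall event.
; Each SpawnWall call spawns the class at CurrentIndex using the Arrow component's world transform, then advances the index with modulo wrapping, cycling through the pool in order.
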(event Custom|SpawnWall
  (bind _enemypool (Variables|Default|GetEnemyPool))
  (Game|SpawnActorfromClass (Utilities|Array|Get(acopy) _enemypool (stale _output_get)) (Transformation|GetWorldTransform (Variables|Default|GetArrow)) "Undefined" "MultiplyWithRoot" 0 0)
  (bind _output_get (Variables|Default|SetCurrentIndex (Math|Integer|%(Integer) (+ (Variables|Default|GetCurrentIndex) 1) (Utilities|Array|Length _enemypool)))))

(event EventBeginPlay
  (Utilities|Time|SetTimerbyEvent (delegate Custom|SpawnWall) 3.0 true))

(fn ConstructionScript)