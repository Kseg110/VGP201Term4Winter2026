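; BP_GameManager is a game manager Blueprint that sets up the game menu and player input when play begins.
; On BeginPlay it prints debug messages, creates WBP_GameMenu, stores a reference and adds it to the viewport.
; It then switches the first player controller to game-only input and hides the mouse cursor.
; TriggerGameOver takes a final score but is an empty stub.
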(event Custom|TriggerGameOver
  (params (FinalScore :type Float%20%28double-precision%29)))

(event EventBeginPlay
  (Development|PrintString "Hello World" true true "(R=0.000000,G=0.660000,B=1.000000,A=1.000000)" 5.0)
  (Development|PrintString "Spawning BP_GameManager" true true "(R=0.000000,G=0.660000,B=1.000000,A=1.000000)" 5.0)
  (CallFunction|SpawnGameMenu)
  (CallFunction|SetInputtoGame))

(event EventTick
  (params (DeltaSeconds :type Float%20%28single-precision%29)))

(fn ConstructionScript)

(fn SpawnGameMenu
  (bind _returnvalue (UserInterface|CreateWidget "/Game/MainMenu/GUI/WBP_GameMenu.WBP_GameMenu_C"))
  (bind _output_get (Variables|Default|SetGameMenuRef _returnvalue))
  (UserInterface|Viewport|AddtoViewport _output_get 0))

(fn SetInputtoGame
  (bind _returnvalue (Game|GetPlayerController 0))
  (Input|SetInputModeGameOnly _returnvalue false)
  (Variables|/Script/Engine.PlayerController|SetbShowMouseCursor _returnvalue false))