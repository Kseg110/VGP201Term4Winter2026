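; BP_EnemyHurdleUp is an enemy hurdle obstacle that hurts the player on contact.
; BeginPlay initializes its own health component with a very large health pool.
; When its Box overlaps a BP_Player, it applies fixed damage through the player's health component, prints the remaining health on screen, then destroys itself.
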(event OnComponentBeginOverlap(Box)
  (params (OverlappedComponent :type Primitive%20Component%20Object%20Reference) (OtherActor :type Actor%20Object%20Reference) (OtherComp :type Primitive%20Component%20Object%20Reference) (OtherBodyIndex :type Integer) (bFromSweep :type Boolean) (SweepResult :type Hit%20Result%20Structure%20%28by%20ref%29))
  (bind _asbp_player (Utilities|Casting|CastToBP_Player OtherActor))
  (Default|CustomDamage (Variables|/Game/Player/BP_Player.BP_Player_C|GetAC_HealthComponent _asbp_player) 25.0)
  (Development|PrintString (Utilities|String|ToString(Float) (Default|GetHealth (Variables|/Game/Player/BP_Player.BP_Player_C|GetAC_HealthComponent _asbp_player))) true true "(R=1.000000,G=0.177888,B=0.187821,A=1.000000)" 5.0)
  (Actor|DestroyActor))

(event EventBeginPlay
  (Default|Init (Variables|Default|GetAC_HealthComponent) 1e+04 0.0 1e+04))

(fn ConstructionScript
  (|CallParentFunction))