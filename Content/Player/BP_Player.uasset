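; Player character Blueprint for a shooter, handling look, movement, jump, a sideways dash launch and gun fire.
; BeginPlay spawns and attaches the starting gun and adds the game menu widget.
; Firing reads fire-rate delay and range through BPI_gun, line traces from the camera, notifies the gun on any hit and damages actors with AC_HealthComponent.
; The player's own health initialization is present but unwired.
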(event EventBeginPlay
  (Development|PrintString "Spawned Player" true true "(R=0.362511,G=1.000000,B=0.347398,A=1.000000)" 5.0)
  (CallFunction|SpawnGun (Variables|Default|GetStartingGun))
  (Input|SetInputModeGameOnly (Game|GetPlayerController 0) false)
  (bind _returnvalue (UserInterface|CreateWidget "/Game/MainMenu/GUI/WBP_GameMenu.WBP_GameMenu_C"))
  (UserInterface|Viewport|AddtoViewport _returnvalue 0))

(event Input|ActionEvents|InputActionJump
  (params (Key :type Key%20Structure :default "None"))
  ;[0.15 0.15 0.15 0.5] Jump Logic
  (:Pressed
    (Character|Jump)))

(event Input|AxisEvents|InputAxisMoveForward
  (params (AxisValue :type Float%20%28single-precision%29))
  ;[0.15 0.15 0.15 0.5] Move Logic
  (Pawn|Input|AddMovementInput (Transformation|GetActorForwardVector) AxisValue false))

(event Input|AxisEvents|InputAxisHorizontal
  (params (AxisValue :type Float%20%28single-precision%29))
  ;[0.15 0.15 0.15 0.5] Camera Logic
  (Pawn|Input|AddControllerYawInput AxisValue))

(event Input|AxisEvents|InputAxisVertical
  (params (AxisValue :type Float%20%28single-precision%29))
  ;[0.15 0.15 0.15 0.5] Camera Logic
  (Pawn|Input|AddControllerPitchInput AxisValue))

(event Input|AxisEvents|InputAxisFire1
  (params (AxisValue :type Float%20%28single-precision%29))
  ;[0.15 0.15 0.15 0.5] Shooting Logic
  (if (> AxisValue 0.0)
    (Utilities|PlayerShooting)
    (Development|PrintString "Shooting" true true "(R=1.000000,G=0.214249,B=0.718978,A=1.000000)" 4.0)))

(event Input|AxisEvents|InputAxisMoveRight
  (params (AxisValue :type Float%20%28single-precision%29))
  ;[0.15 0.15 0.15 0.5] Move Logic
  (Pawn|Input|AddMovementInput (Transformation|GetActorRightVector) AxisValue false))

(event Input|KeyboardEvents|LeftShift
  (params (Key :type Key%20Structure :default "None"))
  ;[0.15 0.15 0.15 0.5] Dash Logic
  (:Pressed
    (CallFunction|Dash)))

(fn ConstructionScript)

(fn SpawnGun
  (params (GunToSpawn :type Actor%20Class%20Reference))
  (bind _returnvalue (Game|SpawnActorfromClass GunToSpawn (Math|Transform|MakeTransform "0, 0, 0") "Undefined" "MultiplyWithRoot" 0 0))
  (bind _output_get (Variables|Default|SetGunRef _returnvalue))
  (Transformation|AttachComponentToComponent _output_get (Variables|Default|GetGunSpawnPoint) "None" "SnapToTarget" "SnapToTarget" "SnapToTarget" true)
  (bind _asbpi_gun (Utilities|Casting|CastToBPI_gun _output_get)
    (:then
      (Variables|Default|SetGunInterfaceRef _asbpi_gun))
    (:CastFailed
      _))
  (return _output_get))

(fn CalculateShoot
  (bind _returnvalue (Game|GetPlayerCameraManager 0))
  (bind _returnvalue_2 (Camera|GetCameraLocation _returnvalue))
  (bind _distance (Default|GetDistance (Variables|Default|GetGunInterfaceRef)))
  (return _returnvalue_2 (+ _returnvalue_2 (* (Transformation|GetActorForwardVector _returnvalue) _distance))))

(fn Dash
  (Character|LaunchCharacter (* (* (Transformation|GetActorRightVector) (Input|AxisValues|GetMoveRight)) 3e+03) true false))